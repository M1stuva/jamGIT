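; BP_GoingDownObject is a configurable platform that moves toward an end location while the third-person character overlaps its Box.
; The MovePlatform timeline lerps MainPlatform's relative location over DurationInSeconds, reversing when the character leaves.
; The construction script applies the mesh and scale to both the platform and an end-position reference mesh, but applies Rotation only to the reference.
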(event OnComponentBeginOverlap(Box)
  (params (OverlappedComponent :type Primitive%20Component%20Object%20Reference) (OtherActor :type Actor%20Object%20Reference) (OtherComp :type Primitive%20Component%20Object%20Reference) (OtherBodyIndex :type Integer) (bFromSweep :type Boolean) (SweepResult :type Hit%20Result%20Structure%20%28by%20ref%29))
  (Utilities|Casting|CastToBP_ThirdPersonCharacter OtherActor)
  (Components|Timeline|SetPlayRate (Variables|Default|GetMovePlatform) (/ 1.0 (Variables|Default|GetDurationInSeconds)))
  (bind _move_track (Timeline|MovePlatform Play)
    (:Update
      (Transformation|SetRelativeLocation (Variables|Default|GetMainPlatform) (Math|Vector|Lerp(Vector) (Variables|Default|GetStartLocation) (Variables|Default|GetEnd%20Location) _move_track) false false))))

(event OnComponentEndOverlap(Box)
  (params (OverlappedComponent :type Primitive%20Component%20Object%20Reference) (OtherActor :type Actor%20Object%20Reference) (OtherComp :type Primitive%20Component%20Object%20Reference) (OtherBodyIndex :type Integer))
  (Utilities|Casting|CastToBP_ThirdPersonCharacter OtherActor)
  (Components|Timeline|SetPlayRate (Variables|Default|GetMovePlatform) (/ 1.0 (Variables|Default|GetDurationInSeconds)))
  (bind _move_track (Timeline|MovePlatform Reverse)
    (:Update
      (Transformation|SetRelativeLocation (Variables|Default|GetMainPlatform) (Math|Vector|Lerp(Vector) (Variables|Default|GetStartLocation) (Variables|Default|GetEnd%20Location) _move_track) false false))))

(event EventBeginPlay
  (Variables|Default|SetStartLocation (Variables|/Script/Engine.SceneComponent|GetRelativeLocation (Variables|Default|GetMainPlatform))))

(fn ConstructionScript
  (bind _mainplatform (Variables|Default|GetMainPlatform))
  (bind _endplatformreference (Variables|Default|GetEndPlatformReference))
  (bind _platformmesh (Variables|Default|GetPlatformMesh))
  (Components|StaticMesh|SetStaticMesh _mainplatform _platformmesh)
  (Components|StaticMesh|SetStaticMesh _endplatformreference _platformmesh)
  (Transformation|SetRelativeScale3D _mainplatform (Variables|Default|GetScale))
  (Transformation|SetRelativeRotation _endplatformreference (Variables|Default|GetRotation) false false)
  (Transformation|SetRelativeLocation _endplatformreference (Variables|Default|GetEnd%20Location) false false))